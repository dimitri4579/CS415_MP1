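; BP_Tunnel is a tunnel segment with a rotating holed wall that the player must pass through.
; RandomizeWall picks one of four hole meshes and a random roll, while Tick keeps the wall spinning.
; Wall contact flags a hit; overlapping the trigger has TunnelSpawner spawn another tunnel and destroys this one.
; A flagged hit costs health and can trigger death and restart, while a clean pass raises score and forward speed.
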(event OnComponentBeginOverlap(TriggerZone)
  (params (OverlappedComponent :type Primitive%20Component%20Object%20Reference) (OtherActor :type Actor%20Object%20Reference) (OtherComp :type Primitive%20Component%20Object%20Reference) (OtherBodyIndex :type Integer) (bFromSweep :type Boolean) (SweepResult :type Hit%20Result%20Structure%20%28by%20ref%29))
  (bind _asbp_player (Utilities|Casting|CastToBP_Player OtherActor))
  (Default|SpawnTunnelatSpawnPoint (Variables|Default|GetTunnelSpawner))
  (Actor|DestroyActor)
  (if (Variables|Default|GetHitWall)
    (CallFunction|ProcessHit _asbp_player)
    (Variables|Default|SetHitWall false)
    (else
      (CallFunction|IncrementScore _asbp_player))))

(event OnComponentHit(WallMesh)
  (params (HitComponent :type Primitive%20Component%20Object%20Reference) (OtherActor :type Actor%20Object%20Reference) (OtherComp :type Primitive%20Component%20Object%20Reference) (NormalImpulse :type Vector :default "0, 0, 0") (Hit :type Hit%20Result%20Structure%20%28by%20ref%29))
  (Utilities|Casting|CastToBP_Player OtherActor)
  (Variables|Default|SetHitWall true))

(event EventBeginPlay)

(event EventTick
  (params (DeltaSeconds :type Float%20%28single-precision%29))
  (Transformation|AddLocalRotation (Variables|Default|GetWallMesh) (Math|Rotator|MakeRotator (* DeltaSeconds (Variables|Default|GetRotateSpeed)) 0.0 0.0) false false))

(fn ConstructionScript)

(fn RandomizeWall
  (Components|StaticMesh|SetStaticMesh (Variables|Default|GetWallMesh) (Utilities|Select :Index (Math|Random|RandomIntegerinRange 0 3) :Option%200 "/Game/InfiniteMatrix/Meshes/SM_Hole_01.SM_Hole_01" :Option%201 "/Game/InfiniteMatrix/Meshes/SM_Hole_02.SM_Hole_02" :Option%202 "/Game/InfiniteMatrix/Meshes/SM_Hole_03.SM_Hole_03" :Option%203 "/Game/InfiniteMatrix/Meshes/SM_Hole_04.SM_Hole_04"))
  (Transformation|AddLocalRotation (Variables|Default|GetWallMesh) (Math|Rotator|MakeRotator (Math|Random|RandomFloatinRange 0.0 3.6e+02) 0.0 0.0) false false))

(fn ProcessHit
  (params (Player :type BP%20Player%20Object%20Reference))
  (bind _output_get (Variables|/Game/InfiniteMatrix/Blueprints/BP_Player.BP_Player_C|SetHealth Player (- (Variables|/Game/InfiniteMatrix/Blueprints/BP_Player.BP_Player_C|GetHealth Player) 1e+01)))
  (Default|UpdateHealthBar (Variables|/Game/InfiniteMatrix/Blueprints/BP_Player.BP_Player_C|GetWB%20Healthbar Player) _output_get)
  (if (<= _output_get 0.0)
    (Variables|/Game/InfiniteMatrix/Blueprints/BP_Player.BP_Player_C|SetIsDead Player true)
    (Default|DisplayRestart Player)))

(fn IncrementScore
  (params (player :type BP%20Player%20Object%20Reference))
  (if (not (Variables|Default|GetHitWall))
    (Variables|/Game/InfiniteMatrix/Blueprints/BP_Player.BP_Player_C|SetScore player (+ (Variables|/Game/InfiniteMatrix/Blueprints/BP_Player.BP_Player_C|GetScore player) 1))
    (Variables|/Game/InfiniteMatrix/Blueprints/BP_Player.BP_Player_C|SetForwardSpeed player (+ (Variables|/Game/InfiniteMatrix/Blueprints/BP_Player.BP_Player_C|GetForwardSpeed player) 75.0))))